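; BP_CubeCleaner is a wandering physics cube that switches between hostile and non-hostile on contact with other cubes of its class.
; Touching a cleaner turns a non-hostile cube hostile, while a non-hostile cube converts any hostile non-cleaner it hits.
; Each conversion swaps the material and lowers or raises points through BP_GM.
; Tick feeds a random Delay that fires horizontal velocity-change impulses at irregular intervals.
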(event EventTick
  (params (DeltaSeconds :type Float%20%28single-precision%29))
  (bind _minshift (Variables|Default|GetminShift))
  (bind _maxshift (Variables|Default|GetmaxShift))
  ;[1 1 1] Random movement
  (Utilities|FlowControl|Delay (Math|Random|RandomFloatinRange 0.0 1.0))
  (Physics|AddImpulse (Variables|Default|GetCube) (* (Variables|Default|GetSpeed) (Math|Vector|MakeVector (Math|Random|RandomFloatinRange _minshift _maxshift) (Math|Random|RandomFloatinRange _minshift _maxshift) 0.0)) "None" true))

(event Collision|EventHit
  (params (MyComp :type Primitive%20Component%20Object%20Reference) (Other :type Actor%20Object%20Reference) (OtherComp :type Primitive%20Component%20Object%20Reference) (bSelfMoved :type Boolean) (HitLocation :type Vector :default "0, 0, 0") (HitNormal :type Vector :default "0, 0, 0") (NormalImpulse :type Vector :default "0, 0, 0") (Hit :type Hit%20Result%20Structure%20%28by%20ref%29))
  (bind _returnvalue (Game|GetGameMode))
  ;[1 1 1] repaint on hit
  (bind _asbp_cube_cleaner (Utilities|Casting|CastToBP_CubeCleaner Other))
  (Audio|PlaySound2D "/Game/Sounds/HitSound_Cue.HitSound_Cue" 1.0 1.0 0.0 0 0)
  (if (Variables|BP_CubeCleaner_C|GetisCleaner _asbp_cube_cleaner)
    (if (not (Variables|Default|GetisHostile))
      (Variables|Default|SetisHostile true)
      (Rendering|Material|SetMaterial (Variables|Default|GetCube) 0 "/Game/Materials/M_Cube.M_Cube")
      (bind _asbp_gm (Utilities|Casting|CastToBP_GM _returnvalue))
      (Default|PtsDecrease _asbp_gm))
    (elif (Variables|BP_CubeCleaner_C|GetisHostile _asbp_cube_cleaner)
      (if (not (Variables|Default|GetisHostile))
        (Variables|BP_CubeCleaner_C|SetisHostile _asbp_cube_cleaner false)
        (Rendering|Material|SetMaterial (Variables|BP_CubeCleaner_C|GetCube _asbp_cube_cleaner) 0 "/Game/Materials/M_Player.M_Player")
        (bind _asbp_gm_2 (Utilities|Casting|CastToBP_GM _returnvalue))
        (Default|PtsIncrease _asbp_gm_2)))))

(fn ConstructionScript)