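; Player-controlled rolling character that repaints hostile cubes on contact to earn points.
; Enhanced Input drives camera look and movement, which applies camera-relative angular impulses to the physics capsule as velocity changes.
; Hitting any BP_CubeCleaner plays a sound; hostile ones become non-hostile, take the player material and report points to BP_GM, with cleaner cubes also losing cleaner status and notifying it.
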(event Input|EnhancedActionEvents|EnhancedInputActionIA_Movement
  (params (ActionValue :type Vector%202D%20Structure) (ElapsedSeconds :type Float%20%28double-precision%29) (TriggeredSeconds :type Float%20%28double-precision%29) (InputAction :type Input%20Action%20Object%20Reference :default "/Game/Blueprints/IA_Movement.IA_Movement"))
  (bind _returnvalue (Pawn|GetControlRotation :!class /Script/Engine.Pawn))
  ;[1 1 1] Movement
  (:Triggered
    (Class|PrimitiveComponent|AddAngularImpulseinDegrees (Variables|Collision|GetCapsuleComponent) (* (Variables|Default|GetSpeed) (.x ActionValue) (Math|Vector|GetForwardVector (Math|Rotator|MakeRotator 0.0 0.0 (.yaw (Pawn|GetControlRotation :!class /Script/Engine.Pawn))))) "None" true)
    (Class|PrimitiveComponent|AddAngularImpulseinDegrees (Variables|Collision|GetCapsuleComponent) (* (Variables|Default|GetSpeed) (.y ActionValue) (Math|Vector|GetRightVector (Math|Rotator|MakeRotator (.roll _returnvalue) 0.0 (.yaw _returnvalue)))) "None" true)))

(event Input|EnhancedActionEvents|EnhancedInputActionIA_Look
  (params (ActionValue :type Vector%202D%20Structure) (ElapsedSeconds :type Float%20%28double-precision%29) (TriggeredSeconds :type Float%20%28double-precision%29) (InputAction :type Input%20Action%20Object%20Reference :default "/Game/Blueprints/IA_Look.IA_Look"))
  ;[1 1 1] CameraRotation
  (:Triggered
    (Pawn|Input|AddControllerYawInput (.x ActionValue))
    (Pawn|Input|AddControllerPitchInput (.y ActionValue))))

(event EventBeginPlay
  (bind _asplayer_controller (Utilities|Casting|CastToPlayerController (Pawn|GetController)))
  (Utilities|IsValid (PlayerController|LocalPlayerSubsystems|GetEnhancedInputLocalPlayerSubsystem _asplayer_controller)
    (:Is%20Valid
      (Input|AddMappingContext (PlayerController|LocalPlayerSubsystems|GetEnhancedInputLocalPlayerSubsystem _asplayer_controller) "/Game/Blueprints/IMC_Main.IMC_Main" 0 "(bIgnoreAllPressedKeysUntilRelease=True,bForceImmediately=False)"))))

(event Collision|EventHit
  (params (MyComp :type Primitive%20Component%20Object%20Reference) (Other :type Actor%20Object%20Reference) (OtherComp :type Primitive%20Component%20Object%20Reference) (bSelfMoved :type Boolean) (HitLocation :type Vector :default "0, 0, 0") (HitNormal :type Vector :default "0, 0, 0") (NormalImpulse :type Vector :default "0, 0, 0") (Hit :type Hit%20Result%20Structure%20%28by%20ref%29))
  ;[1 1 1] Repaint on hit
  (bind _asbp_cube_cleaner (Utilities|Casting|CastToBP_CubeCleaner Other))
  (Audio|PlaySound2D "/Game/Sounds/HitSound_Cue.HitSound_Cue" 1.0 1.0 0.0 0 0)
  (if (Variables|/Game/Blueprints/BP_CubeCleaner.BP_CubeCleaner_C|GetisHostile _asbp_cube_cleaner)
    (Variables|/Game/Blueprints/BP_CubeCleaner.BP_CubeCleaner_C|SetisHostile _asbp_cube_cleaner false)
    (Rendering|Material|SetMaterial (Variables|/Game/Blueprints/BP_CubeCleaner.BP_CubeCleaner_C|GetCube _asbp_cube_cleaner) 0 "/Game/Materials/M_Player.M_Player")
    (bind _asbp_gm (Utilities|Casting|CastToBP_GM (Game|GetGameMode)))
    (Default|PtsIncrease _asbp_gm)
    (if (Variables|/Game/Blueprints/BP_CubeCleaner.BP_CubeCleaner_C|GetisCleaner _asbp_cube_cleaner)
      (Variables|/Game/Blueprints/BP_CubeCleaner.BP_CubeCleaner_C|SetisCleaner _asbp_cube_cleaner false)
      (Default|CleanerRepaint _asbp_gm))))

(fn ConstructionScript)