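; BP_GM tracks progress in a cube-repainting game and drives its HUD and win condition.
; On BeginPlay it creates the BP_GameUI widget, then its custom events update point and cleaner counters and write them straight to that widget.
; Each point gain runs an exact-match check against PointsToWin, which plays a win sound and sets the UI's Win value on success.
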(event Custom|PtsIncrease
  (bind _output_get (Variables|Default|SetCurrentPoints (+ 1 (Variables|Default|GetCurrentPoints))))
  (Variables|/Game/Blueprints/BP_GameUI.BP_GameUI_C|SetRepaintedCubes (Variables|Default|GetUI) _output_get)
  (CallFunction|Win))

(event Custom|Win
  (if (== (Variables|Default|GetCurrentPoints) (Variables|Default|GetPointsToWin))
    (Audio|PlaySound2D "/Game/Sounds/YouWinSound_Cue.YouWinSound_Cue" 1.0 1.0 0.0 0 0)
    (Variables|/Game/Blueprints/BP_GameUI.BP_GameUI_C|SetWin (Variables|Default|GetUI) 1.0)))

(event Custom|PtsDecrease
  (bind _output_get (Variables|Default|SetCurrentPoints (+ (Variables|Default|GetCurrentPoints) -1)))
  (Variables|/Game/Blueprints/BP_GameUI.BP_GameUI_C|SetRepaintedCubes (Variables|Default|GetUI) _output_get))

(event Custom|CleanerRepaint
  (bind _output_get (Variables|Default|SetCleanersAlive (+ (Variables|Default|GetCleanersAlive) -1)))
  (Variables|/Game/Blueprints/BP_GameUI.BP_GameUI_C|SetCubeCleaners (Variables|Default|GetUI) _output_get))

(event EventBeginPlay
  (bind _returnvalue (UserInterface|CreateWidget "/Game/Blueprints/BP_GameUI.BP_GameUI_C"))
  (bind _output_get (Variables|Default|SetUI _returnvalue))
  (UserInterface|Viewport|AddtoViewport _output_get 0))

(fn ConstructionScript)