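; BP_Cube is a randomly moving cube that spreads the player material on contact to score points.
; When a player-colored cube hits another BP_Cube, it plays a sound, repaints that cube if needed and calls PtsIncrease on BP_GM.
; The material itself serves as the ownership state.
; A random Delay on Tick spaces out horizontal, mass-independent impulses scaled by Speed.
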(event Collision|EventHit
  (params (MyComp :type Primitive%20Component%20Object%20Reference) (Other :type Actor%20Object%20Reference) (OtherComp :type Primitive%20Component%20Object%20Reference) (bSelfMoved :type Boolean) (HitLocation :type Vector :default "0, 0, 0") (HitNormal :type Vector :default "0, 0, 0") (NormalImpulse :type Vector :default "0, 0, 0") (Hit :type Hit%20Result%20Structure%20%28by%20ref%29))
  ;[1 1 1] Repaint on hit
  (if (== (Rendering|Material|GetMaterial (Variables|Default|GetCube) 0) "/Game/Materials/M_Player.M_Player")
    (bind _asbp_cube (Utilities|Casting|CastToBP_Cube Other))
    (Audio|PlaySound2D "/Game/Sounds/HitSound_Cue.HitSound_Cue" 1.0 1.0 0.0 0 0)
    (if (!= (Rendering|Material|GetMaterial (Variables|BP_Cube_C|GetCube _asbp_cube) 0) "/Game/Materials/M_Player.M_Player")
      (Rendering|Material|SetMaterial (Variables|BP_Cube_C|GetCube _asbp_cube) 0 "/Game/Materials/M_Player.M_Player")
      (bind _asbp_gm (Utilities|Casting|CastToBP_GM (Game|GetGameMode)))
      (Default|PtsIncrease _asbp_gm))))

(event EventTick
  (params (DeltaSeconds :type Float%20%28single-precision%29))
  (bind _min (Variables|Default|Getmin))
  (bind _max (Variables|Default|Getmax))
  ;[1 1 1] Random movement
  (Utilities|FlowControl|Delay (Math|Random|RandomFloatinRange 0.0 1.0))
  (Physics|AddImpulse (Variables|Default|GetCube) (* (Variables|Default|GetSpeed) (Math|Vector|MakeVector (Math|Random|RandomFloatinRange _min _max) (Math|Random|RandomFloatinRange _min _max) 0.0)) "None" true))

(fn ConstructionScript)